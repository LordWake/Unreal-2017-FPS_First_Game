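; Power-up actor placed in levels, with Life, Speed and Weapon boxes plus green, yellow and red lights.
; BeginPlay stores these components in variables, then calls CheckMyBox.
; Any box overlapped by BP_MyMainPlayer calls the same PlayerRequestPowerUp, passing no type or player.
; Both functions are defined outside this Blueprint, so it only wires components and overlap events to that logic.
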(event `self.ReceiveBeginPlay`
  (`|ExecutionSequence`
    (:`then_0`
      (set `self.lifeBox` (`self.BoxLife`))
      (set `self.myGreenLight` (`self.GreenLight`)))
    (:`then_1`
      (set `self.speedBox` (`self.BoxSpeed`))
      (set `self.myYellowLight` (`self.YellowLight`)))
    (:`then_2`
      (set `self.weaponBox` (`self.BoxWeapon`))
      (set `self.myRedLight` (`self.Red Light`)))
    (:`then_3`
      (`self.CheckMyBox`))))

(event `self.BoxLife.OnComponentBeginOverlap`
  (params (OverlappedComponent :type "PrimitiveComponent Object Reference") (OtherActor :type "Actor Object Reference") (OtherComp :type "PrimitiveComponent Object Reference") (OtherBodyIndex :type Integer) (bFromSweep :type Boolean) (SweepResult :type "HitResult Structure (by ref)"))
  (cast `/Game/Blueprints/Levels/ActorsOnScene/BP_MyMainPlayer` OtherActor)
  (`self.PlayerRequestPowerUp`))

(event `self.BoxSpeed.OnComponentBeginOverlap`
  (params (OverlappedComponent :type "PrimitiveComponent Object Reference") (OtherActor :type "Actor Object Reference") (OtherComp :type "PrimitiveComponent Object Reference") (OtherBodyIndex :type Integer) (bFromSweep :type Boolean) (SweepResult :type "HitResult Structure (by ref)"))
  (cast `/Game/Blueprints/Levels/ActorsOnScene/BP_MyMainPlayer` OtherActor)
  (`self.PlayerRequestPowerUp`))

(event `self.BoxWeapon.OnComponentBeginOverlap`
  (params (OverlappedComponent :type "PrimitiveComponent Object Reference") (OtherActor :type "Actor Object Reference") (OtherComp :type "PrimitiveComponent Object Reference") (OtherBodyIndex :type Integer) (bFromSweep :type Boolean) (SweepResult :type "HitResult Structure (by ref)"))
  (cast `/Game/Blueprints/Levels/ActorsOnScene/BP_MyMainPlayer` OtherActor)
  (`self.PlayerRequestPowerUp`))

(fn `UserConstructionScript`)