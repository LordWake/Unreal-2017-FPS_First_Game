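; Enemy turret actor that reacts to player distance and takes damage from player bullets.
; BeginPlay assigns particle and audio assets for damage, shots and death, and Tick feeds player distance to CheckDistanceToPlayer.
; Body overlaps with BP_PlayerBullet or BP_RiflePlayerBullet call TakeEnemyDamage, with rifle bullets hitting harder.
; Tick also polls IsDead and destroys the turret after a short delay; the combat logic itself lives outside these graphs.
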(event `self.ReceiveBeginPlay`
  (`|ExecutionSequence`
    (:`then_0`
      (set `self.damageParticle` (`self.FireDamageEnemy`)))
    (:`then_1`
      (set `self.shotParticle` (`self.MuzzleFlash`)))
    (:`then_2`
      (set `self.deadParticle` (`self.TurretDead`)))
    (:`then_3`
      (set `self.damageAudio` (`self.Damage`)))
    (:`then_4`
      (set `self.explosionAudio` (`self.Explosion`)))
    (:`then_5`
      (set `self.shotAudio` (`self.Shot`)))))

(event `self.ReceiveTick`
  (params (DeltaSeconds :type "Float (single-precision)"))
  (`|ExecutionSequence`
    (:`then_0`
      (`self.CheckDistanceToPlayer` (`self.GetDistanceTo` (`GameplayStatics.GetPlayerCharacter` 0))))
    (:`then_1`
      (if (== (`self.isDead`) true)
        (`KismetSystemLibrary.Delay` 0.5)
        (`self.K2_DestroyActor`)))))

(event `self.Body.OnComponentBeginOverlap`
  (params (OverlappedComponent :type "PrimitiveComponent Object Reference") (OtherActor :type "Actor Object Reference") (OtherComp :type "PrimitiveComponent Object Reference") (OtherBodyIndex :type Integer) (bFromSweep :type Boolean) (SweepResult :type "HitResult Structure (by ref)"))
  (`|ExecutionSequence`
    (:`then_0`
      (cast `/Game/Blueprints/Levels/ActorsOnScene/BP_PlayerBullet` OtherActor)
      (`self.TakeEnemyDamage` 1.0))
    (:`then_1`
      (cast `/Game/Blueprints/Levels/ActorsOnScene/BP_RiflePlayerBullet` OtherActor)
      (`self.TakeEnemyDamage` 2.0))))

(fn `UserConstructionScript`)