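; BP_MyMainPlayer is the player Blueprint, wiring components to variables and reacting to enemy bullet hits.
; On BeginPlay it stores its guns, muzzle flashes, lasers, shields and audio components in variables.
; Capsule overlaps cast the other actor to each bullet type: normal bullets deal damage, gun-less bullets call GunLess, and slow bullets call FreezeMyPlayer.
; The logic behind those calls is defined outside these graphs.
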(event `self.ReceiveBeginPlay`
  (`|ExecutionSequence`
    (:`then_0`
      (set `self.myGun` (`self.Gun`)))
    (:`then_1`
      (set `self.myRifle` (`self.Rifle`)))
    (:`then_2`
      (set `self.gunMuzzle` (`self.GunFlash`)))
    (:`then_3`
      (set `self.rifleMuzzle` (`self.RifleFlash`)))
    (:`then_4`
      (set `self.myShield` (`self.Shield`)))
    (:`then_5`
      (set `self.rifleLaser` (`self.Cylinder`)))
    (:`then_6`
      (set `self.gunLaser` (`self.StaticMesh`)))
    (:`then_7`
      (set `self.freezeShield` (`self.OnFreeze`)))
    (:`then_8`
      (set `self.damageAudio` (`self.Damage`)))
    (:`then_9`
      (set `self.powerUpAudio` (`self.PowerUp`)))
    (:`then_10`
      (set `self.gunAudio` (`self.GunAudioComponent`)))
    (:`then_11`
      (set `self.rifleAudio` (`self.RifleAudioComponent`)))))

(event `self.CapsuleComponent.OnComponentBeginOverlap`
  (params (OverlappedComponent :type "PrimitiveComponent Object Reference") (OtherActor :type "Actor Object Reference") (OtherComp :type "PrimitiveComponent Object Reference") (OtherBodyIndex :type Integer) (bFromSweep :type Boolean) (SweepResult :type "HitResult Structure (by ref)"))
  (`|ExecutionSequence`
    (:`then_0`
      (cast `/Game/Blueprints/Levels/ActorsOnScene/BP_EnemyBullet` OtherActor)
      (`self.TakePlayerDamage` 1.0))
    (:`then_1`
      (cast `/Game/Blueprints/Levels/ActorsOnScene/BP_GunLessBullet` OtherActor)
      (`self.GunLess`))
    (:`then_2`
      (cast `/Game/Blueprints/Levels/ActorsOnScene/BP_SlowBullet` OtherActor)
      (`self.FreezeMyPlayer`))))

(fn `UserConstructionScript`)