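; BP_WoodStock is a boss enemy actor with a rifle, laser shield and levitation effect.
; On BeginPlay it assigns its particle, audio, weapon and shield components to variables, apparently for inherited boss logic to use.
; Skeletal mesh overlaps with player bullets call TakeEnemyDamage, with rifle bullets dealing more damage than standard ones.
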(event `self.ReceiveBeginPlay`
  (set `self.damageParticle` (`self.BossDamage`))
  (set `self.shotParticle` (`self.Shot`))
  (set `self.myWeapon` (`self.Rifle`))
  (set `self.shield` (`self.ShieldLaser`))
  (set `self.levitateParticle` (`self.BossLevitate`))
  (set `self.damageAudio` (`self.Damage`))
  (set `self.shotAudio` (`self.ShotAudioComponent`)))

(event `self.SkeletalMesh.OnComponentBeginOverlap`
  (params (OverlappedComponent :type "PrimitiveComponent Object Reference") (OtherActor :type "Actor Object Reference") (OtherComp :type "PrimitiveComponent Object Reference") (OtherBodyIndex :type Integer) (bFromSweep :type Boolean) (SweepResult :type "HitResult Structure (by ref)"))
  (`|ExecutionSequence`
    (:`then_0`
      (cast `/Game/Blueprints/Levels/ActorsOnScene/BP_PlayerBullet` OtherActor)
      (`self.TakeEnemyDamage` 0.25))
    (:`then_1`
      (cast `/Game/Blueprints/Levels/ActorsOnScene/BP_RiflePlayerBullet` OtherActor)
      (`self.TakeEnemyDamage` 0.5))))

(fn `UserConstructionScript`)